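; GA_BPTest is a test Gameplay Ability that exercises cost, cooldown and commit handling in GAS, with Korean debug prints.
; On activation, a Sequence checks cost, then cooldown, printing a not-enough-mana or cooldown message and cancelling on failure.
; The last pin commits the ability, then prints an activation message and ends it on success.
; Cancelling does not stop later Sequence pins from executing.
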(event `self.K2_ActivateAbility`
  (`|ExecutionSequence`
    (:`then_0`
      (bind _returnvalue (`self.K2_CheckAbilityCost`))
      (if (not _returnvalue)
        (`KismetSystemLibrary.PrintString` "마나가 부족합니다.")
        (`self.K2_CancelAbility`)))
    (:`then_1`
      (bind _returnvalue_2 (`self.K2_CheckAbilityCooldown`))
      (if (not _returnvalue_2)
        (`KismetSystemLibrary.PrintString` "쿨타임이 아직 멀었습니다.")
        (`self.K2_CancelAbility`)))
    (:`then_2`
      (bind _returnvalue_3 (`self.K2_CommitAbility`))
      (if _returnvalue_3
        (`KismetSystemLibrary.PrintString` "Test 어빌리티 발동")
        (`self.K2_EndAbility`)))))